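; Hydrazine generator that the player toggles with Use, producing power while enabled and fuelled.
; Construction reads the fuel whitelist from the storage chassis's "FuelRule" and caches the input slot reference.
; Tick on authority consumes whitelisted fuel at a set rate and switches Power, with paired DoOnce gates firing Anim and Audio on state changes.
; Timelines move the Sphere vertically through start, running and stop phases, alongside matching attached sounds.
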(event Custom|Anim
  (if (and (Variables|Default|GetIsEnabled) (CallFunction|HasFuel))
    (Utilities|FlowControl|Sequence
      (:then_0
        (bind _off (Timeline|Off Stop)
          (:Update
            (Transformation|SetRelativeLocation (Variables|Default|GetSphere) (Math|Vector|MakeVector 0.0 0.0 _off) false false))
          (:Finished
            (Components|Tick|SetComponentTickEnabled (Variables|Default|GetSphere) false))))
      (:then_1
        (Components|Tick|SetComponentTickEnabled (Variables|Default|GetSphere) true)
        (bind _on (Timeline|On PlayFromStart)
          (:Update
            (Transformation|SetRelativeLocation (Variables|Default|GetSphere) (Math|Vector|MakeVector 0.0 0.0 _on) false false))
          (:Finished
            (bind _running (Timeline|Running PlayFromStart)
              (:Update
                (Transformation|SetRelativeLocation (Variables|Default|GetSphere) (Math|Vector|MakeVector 0.0 0.0 _running) false false)))))))
    (else
      (Utilities|FlowControl|Sequence
        (:then_0
          (Timeline|On Stop))
        (:then_1
          (Timeline|Running Stop))
        (:then_2
          (Timeline|Off PlayFromStart))))))

(event Custom|Audio
  (if (and (Variables|Default|GetIsEnabled) (CallFunction|HasFuel))
    (Audio|Components|Audio|Stop (stale _returnvalue_3))
    (bind _returnvalue (Audio|SpawnSoundAttached "/Game/Mods/UnknownMoons/HydrazineGenerator/Audio/Start.Start" (Variables|Default|GetStaticMeshComponent) "None" "0, 0, 0" "0, 0, 0" "KeepRelativeOffset" true 0.3 1.0 0.0 "/Game/Mods/UnknownMoons/HydrazineGenerator/Audio/StartAtten.StartAtten" 0 false))
    (bind _returnvalue_2 (Audio|SpawnSoundAttached "/Game/Mods/UnknownMoons/HydrazineGenerator/Audio/Running.Running" (Variables|Default|GetStaticMeshComponent) "None" "0, 0, 0" "0, 0, 0" "KeepRelativeOffset" true 0.3 1.0 0.0 "/Game/Mods/UnknownMoons/HydrazineGenerator/Audio/RunningAtten.RunningAtten" 0 false))
    (Audio|Components|Audio|Play _returnvalue 0.0)
    (else
      (Audio|Components|Audio|Stop _returnvalue_2)
      (bind _returnvalue_3 (Audio|SpawnSoundAttached "/Game/Mods/UnknownMoons/HydrazineGenerator/Audio/End.End" (Variables|Default|GetStaticMeshComponent) "None" "0, 0, 0" "0, 0, 0" "KeepRelativeOffset" true 0.3 1.0 0.0 "/Game/Mods/UnknownMoons/HydrazineGenerator/Audio/EndAtten.EndAtten" 0 false))
      (Audio|Components|Audio|Play _returnvalue_3 0.0))))

(event EventTick
  (params (DeltaSeconds :type Float%20%28single-precision%29))
  (Networking|SwitchHasAuthority
    (:Authority
      (if (and (Variables|Default|GetIsEnabled) (CallFunction|HasFuel))
        (for _array_element (Utilities|GetClassDefaults (Variables|Default|GetFuelTypeWhiteList))
          (Class|SlotStatics|TakeItemRateDelta (Variables|Default|GetInput%20slot%20ref) _array_element (Variables|Default|GetConsumisonRate) DeltaSeconds 1.0))
        (Class|PowerComponent|SetEnabled (Variables|Default|GetPower) true)
        (Utilities|FlowControl|DoOnce false :!label _label
          (:Completed
            (CallFunction|Anim)
            (CallFunction|Audio)
            (goto _label_2 Reset)))
        (else
          (Class|PowerComponent|SetEnabled (Variables|Default|GetPower) false)
          (Utilities|FlowControl|DoOnce false :!label _label_2
            (:Completed
              (CallFunction|Anim)
              (CallFunction|Audio)
              (goto _label Reset))))))))

(event Input|ActionEvents|InputActionUse
  (params (Key :type Key%20Structure :default "None"))
  (:Pressed
    (bind _output_get (Variables|Default|SetIsEnabled (not (Variables|Default|GetIsEnabled))))
    (Class|ClickableComponent|SetActiveUseContext (Variables|Default|GetClickableComponent) (select _output_get "UC_TurnOff" "UC_TurnOn"))))

(fn ConstructionScript
  (bind _aswhitelist_organization_rule (Utilities|Casting|CastToWhitelistOrganizationRule (Class|StorageChassisComponent|FindRulebyName (Variables|Default|GetStorageChassis) "FuelRule")))
  (Variables|Default|SetFuelTypeWhiteList (Variables|/Script/Astro.WhitelistOrganizationRule|GetItemTypeWhitelist _aswhitelist_organization_rule))
  (Variables|Default|SetInput%20slot%20ref (Class|ChildSlotComponent|MakeReference (Variables|Default|GetInputSlot))))

(fn HasFuel
  (for _array_element (Utilities|GetClassDefaults (Variables|Default|GetFuelTypeWhiteList))
    (if (Class|SlotStatics|HasItem (Variables|Default|GetInput%20slot%20ref) _array_element)
      (return true)))
  (return false))

(fn GetBodySlotLegacy
  (return (Variables|Default|GetBodySlot)))