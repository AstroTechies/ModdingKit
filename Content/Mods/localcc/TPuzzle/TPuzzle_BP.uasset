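; TPuzzle_BP is a one-time puzzle actor that hosts a TPanel child actor and rewards a win with random loot.
; It binds to the panel's win event and drives the panel's CustomTick each frame.
; On win, the authority disables interaction, spawns an item drawn from LootTable using Count-derived probabilities, and sets DroppedOut.
; A timer drives curve-based panel shrinking before destruction; BeginPlay removes the panel if DroppedOut is already set.
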(event Custom|OnWin
  (bind _clickablecomponent (Variables|Default|GetClickableComponent))
  (Networking|SwitchHasAuthority
    (:Authority
      (Variables|/Script/Astro.ClickableComponent|SetHasUseInteractionByDefault _clickablecomponent false)
      (Components|Activation|SetActive _clickablecomponent false false)
      (bind _returnvalue (Utilities|Time|SetTimerbyEvent (delegate Custom|Finished) 2.0 false 1.0))
      (Variables|Default|SetShrinkTimer _returnvalue)
      (bind _item (CallFunction|GenerateLoot))
      (Class|SlotsComponent|SpawnItemTypeinSlot (Class|ChildSlotComponent|MakeReference (Variables|Default|GetChildSlot)) _item true)
      (Variables|Default|SetDroppedOut true))))

(event Custom|Finished
  (Components|DestroyComponent (Variables|Default|GetChildActor))
  (Variables|Default|SetShrinkTimer ""))

(event EventTick
  (params (DeltaSeconds :type Float%20%28single-precision%29))
  (bind _shrinktimer (Variables|Default|GetShrinkTimer))
  (bind _childactor (Variables|Default|GetChildActor))
  (if (Utilities|IsValid _childactor)
    (if (Utilities|Time|IsValidTimerHandle _shrinktimer)
      (Transformation|SetActorScale3D (Variables|/Script/Engine.ChildActorComponent|GetChildActor _childactor) (Math|Conversions|ToVector(Float) (Math|Curves|GetFloatValue (Variables|Default|GetShrinkAnim) (Math|Float|MapRangeClamped (Class|KismetSystemLibrary|GetTimerElapsedTimeHandle _shrinktimer) 0.0 2.0 0.0 1.0)))))
    (bind _astpanel (Utilities|Casting|CastToTPanel (Variables|/Script/Engine.ChildActorComponent|GetChildActor (Variables|Default|GetChildActor))))
    (Default|CustomTick _astpanel)))

(event EventBeginPlay
  (if (Variables|Default|GetDroppedOut)
    (Components|DestroyComponent (Variables|Default|GetChildActor))
    (else
      (bind _astpanel (Utilities|Casting|CastToTPanel (Variables|/Script/Engine.ChildActorComponent|GetChildActor (Variables|Default|GetChildActor))))
      (EventDispatchers|BindEventtoWin _astpanel (delegate Custom|OnWin))
      (|GenerateProbabilities))))

(fn ConstructionScript)

(fn Win
  (bind _astpanel (Utilities|Casting|CastToTPanel (Variables|/Script/Engine.ChildActorComponent|GetChildActor (Variables|Default|GetChildActor))))
  (Default|CallWin _astpanel))

(fn GenerateLoot
  (LocalVariables|SetNum (Math|Random|RandomFloat))
  (LocalVariables|SetMass 1.0)
  (bind (_array_element _array_index) (Utilities|Array|ForEachLoopwithBreak (Variables|Default|GetProbabilities) :!label _label)
    (:LoopBody
      (if (<= (LocalVariables|GetNum) (/ _array_element (LocalVariables|GetMass)))
        (LocalVariables|SetIndex _array_index)
        (goto _label Break)
        (else
          (LocalVariables|SetMass (- (LocalVariables|GetMass) _array_element)))))
    (:Completed
      (return (.ItemType (Utilities|Struct|BreakItemRecipeIngredient (Utilities|Array|Get(acopy) (Utilities|Struct|BreakRecipe (Variables|Default|GetLootTable)) (LocalVariables|GetIndex))))))))