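; PurpleLavaLamp_BP is the purple variant of a lava lamp actor from the LavaLamp mod.
; On BeginPlay it runs the parent logic, then pushes a fixed Fresnel power and its OuterColor and InnerColor variables into the glass material.
; The inner color also tints the point light, so the glow matches the lamp.
; Tick and the construction script only call the parent.
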(event EventBeginPlay
  (bind _innercolor (Variables|Default|GetInnerColor))
  (bind _glassmaterial (Variables|Default|GetGlassMaterial))
  (|CallParentFunction)
  (Rendering|Material|SetScalarParameterValue _glassmaterial "FresnelPower" 0.820168 :!class /Script/Engine.MaterialInstanceDynamic)
  (Rendering|Material|SetVectorParameterValue _glassmaterial "OuterColor" (Variables|Default|GetOuterColor) :!class /Script/Engine.MaterialInstanceDynamic)
  (Rendering|Material|SetVectorParameterValue _glassmaterial "InnerColor" _innercolor :!class /Script/Engine.MaterialInstanceDynamic)
  (Rendering|Components|Light|SetLightColor (Variables|Default|GetPointLight) _innercolor true))

(event Collision|EventActorBeginOverlap
  (params (OtherActor :type Actor%20Object%20Reference)))

(event EventTick
  (params (DeltaSeconds :type Float%20%28single-precision%29))
  (|CallParentFunction DeltaSeconds))

(fn ConstructionScript
  (|CallParentFunction))