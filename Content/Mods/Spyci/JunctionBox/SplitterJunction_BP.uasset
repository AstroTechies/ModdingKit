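; Junction box splitter Blueprint that shows a live power total on a text render.
; Every Tick it loops over the replicated cable power values in SplitterRepData, summing only cables whose connection direction converts to zero, using a clamped multiplier as the mask.
; It also builds a per-cable breakdown string, but only the total is displayed.
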(event EventBeginPlay
  (|CallParentFunction) ; This node is disabled and will not be called.\nDrag off pins to build functionality.
)

(event Collision|EventActorBeginOverlap
  (params (OtherActor :type Actor%20Object%20Reference)))

(event EventTick
  (params (DeltaSeconds :type Float%20%28single-precision%29))
  (bind _splitterrepdata (Variables|Default|GetSplitterRepData))
  (Variables|Default|SetTotalPower 0.0)
  (Variables|Default|SetTotalPowerText "")
  (for (_array_element _array_index) (.cablerealpowervalues _splitterrepdata)
    (Variables|Default|SetTotalPowerText (Utilities|Text|FormatText "{a} 
{b}: {c} - {d}" (Variables|Default|GetTotalPowerText) _array_element (- 1 (Math|Conversions|ToInteger(Byte) (Utilities|Array|Get(acopy) (.powercableconnectiondirections _splitterrepdata) _array_index))) (* (Math|Integer|Max(Integer) (- 1 (Math|Conversions|ToInteger(Byte) (Utilities|Array|Get(acopy) (.powercableconnectiondirections _splitterrepdata) _array_index)))) _array_element)))
    (Variables|Default|SetTotalPower (+ (Variables|Default|GetTotalPower) (* (Math|Integer|Max(Integer) (- 1 (Math|Conversions|ToInteger(Byte) (Utilities|Array|Get(acopy) (.powercableconnectiondirections _splitterrepdata) _array_index)))) _array_element))))
  (Rendering|Components|TextRender|SetText (Variables|Default|GetTextRender) (Utilities|Text|FormatText "{b}" (Variables|Default|GetTotalPower))))

(fn ConstructionScript
  (|CallParentFunction))