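; Base junction box Blueprint from a mod, whose body color players cycle through a fixed palette with the Use input.
; The construction script builds the palette and a dynamic material instance, tinting its Base Color parameter from ColorIndex.
; Use calls RunOnServer to advance the index with wraparound, and the ColorIndex RepNotify reapplies the color, as does BeginPlay.
; A legacy getter also exposes the BodySlot.
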(event Custom|RunOnServer
  (CallFunction|CycleColor))

(event EventBeginPlay
  (CallFunction|UpdateMaterialColor (Variables|Default|GetColorIndex)))

(event Input|ActionEvents|InputActionUse
  (params (Key :type Key%20Structure :default "None"))
  (:Pressed
    (CallFunction|RunonServer)))

(fn ConstructionScript
  (Variables|Default|SetColorArray (Utilities|Array|MakeArray "(R=0.019608,G=0.019608,B=0.019608,A=1.000000)" "(R=1.000000,G=0.000000,B=0.000000,A=1.000000)" "(R=1.000000,G=0.000000,B=1.000000,A=1.000000)" "(R=0.384314,G=0.000000,B=1.000000,A=1.000000)" "(R=0.000000,G=0.000000,B=1.000000,A=1.000000)" "(R=0.000000,G=0.690196,B=1.000000,A=1.000000)" "(R=0.117647,G=1.000000,B=0.000000,A=1.000000)" "(R=1.000000,G=0.952941,B=0.000000,A=1.000000)" "(R=0.525490,G=0.101961,B=0.000000,A=1.000000)" "(R=1.000000,G=1.000000,B=1.000000,A=1.000000)"))
  (bind _returnvalue (Rendering|Material|CreateDynamicMaterialInstance (Variables|Default|GetStaticMeshComponent) 0 "/Game/Mods/Spyci/JunctionBox/Models/JunctionBoxMaterial.JunctionBoxMaterial" "None" :!class /Script/Engine.PrimitiveComponent))
  (bind _output_get (Variables|Default|SetBoxMaterial _returnvalue))
  (Rendering|Material|SetVectorParameterValue _output_get "Base Color" (Utilities|Array|Get(acopy) (Variables|Default|GetColorArray) (Variables|Default|GetColorIndex)) :!class /Script/Engine.MaterialInstanceDynamic))

(fn UpdateMaterialColor
  (params (ColorIndex :type Integer))
  (Rendering|Material|SetVectorParameterValue (Variables|Default|GetBoxMaterial) "Base Color" (Utilities|Array|Get(acopy) (Variables|Default|GetColorArray) ColorIndex) :!class /Script/Engine.MaterialInstanceDynamic))

(fn OnRepColorIndex
  (CallFunction|UpdateMaterialColor (Variables|Default|GetColorIndex)))

(fn CycleColor
  (if (>= (Variables|Default|GetColorIndex) (- (Utilities|Array|Length (Variables|Default|GetColorArray)) 1))
    (Variables|Default|SetColorIndex 0)
    (else
      (Variables|Default|SetColorIndex (+ (Variables|Default|GetColorIndex) 1))))
  (return (Variables|Default|GetColorIndex)))

(fn GetBodySlotLegacy
  (return (Variables|Default|GetBodySlot)))