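; Hydrazine generator item that burns whitelisted fuel from its input slot to supply power.
; Pressing Use toggles it on or off and swaps the clickable's use prompt between TurnOn and TurnOff.
; Construction caches the input slot and the storage chassis FuelRule whitelist.
; On authority, Tick drains fuel at a delta-scaled rate and enables Power only while switched on and fueled.
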(event EventTick
  (params (DeltaSeconds :type Float%20%28single-precision%29))
  (Networking|SwitchHasAuthority
    (:Authority
      (if (and (Variables|Default|GetIsEnabled) (CallFunction|HasFuel))
        (for _array_element (Utilities|GetClassDefaults (Variables|Default|GetFuelTypeWhiteList))
          (Class|SlotStatics|TakeItemRateDelta (Variables|Default|GetInput%20slot%20ref) _array_element (Variables|Default|GetConsumisonRate) DeltaSeconds 1.0))
        (Class|PowerComponent|SetEnabled (Variables|Default|GetPower) true)
        (else
          (Class|PowerComponent|SetEnabled (Variables|Default|GetPower) false))))))

(event Input|ActionEvents|InputActionUse
  (params (Key :type Key%20Structure :default "None"))
  (:Pressed
    (bind _output_get (Variables|Default|SetIsEnabled (not (Variables|Default|GetIsEnabled))))
    (Class|ClickableComponent|SetActiveUseContext (Variables|Default|GetClickableComponent) (select _output_get "UC_TurnOff" "UC_TurnOn"))))

(fn ConstructionScript
  (bind _aswhitelist_organization_rule (Utilities|Casting|CastToWhitelistOrganizationRule (Class|StorageChassisComponent|FindRulebyName (Variables|Default|GetStorageChassis) "FuelRule")))
  (Variables|Default|SetFuelTypeWhiteList (Variables|/Script/Astro.WhitelistOrganizationRule|GetItemTypeWhitelist _aswhitelist_organization_rule))
  (Variables|Default|SetInput%20slot%20ref (Class|ChildSlotComponent|MakeReference (Variables|Default|GetInputSlot))))

(fn HasFuel
  (for _array_element (Utilities|GetClassDefaults (Variables|Default|GetFuelTypeWhiteList))
    (if (Class|SlotStatics|HasItem (Variables|Default|GetInput%20slot%20ref) _array_element)
      (return true)))
  (return false))

(fn GetBodySlotLegacy
  (return (Variables|Default|GetBodySlot)))