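; Portable atmospheric condenser that, while switched on and powered, produces a selected gas from the current planet's atmosphere into its output slot.
; CheckGases lists gases with nonzero density, and clicking the right capsule cycles the selection through the player's PMActorComponent, with the replicated index updating a text label.
; On the authority, Tick adds items at a rate scaled by power load ratio and gas density.
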(event OnClicked(Capsule_right)
  (params (TouchedComponent :type Primitive%20Component%20Object%20Reference) (ButtonPressed :type Key%20Structure :default "None"))
  (bind _returnvalue (Class|AstroPlayStatics|GetLocalPlayController))
  (bind _self self)
  (bind _gasidx (Variables|Default|GetGasIdx))
  (bind _returnvalue_2 (Actor|GetComponentbyClass _returnvalue "/Game/Mods/atenfyr/PortableMachines/PMActorComponent.PMActorComponent_C"))
  (bind _returnvalue_3 (+ _gasidx 1))
  (CallFunction|CheckGases)
  (Utilities|IsValid _returnvalue_2
    (:Is%20Valid
      (if (>= _returnvalue_3 (Utilities|Array|Length (Variables|Default|GetAvailableGases)))
        (Default|SetGasIdxonOwningClient _returnvalue_2 0 _self)
        (else
          (Default|SetGasIdxonOwningClient _returnvalue_2 _returnvalue_3 _self))))))

(event Custom|SetEnabled
  (params (NewEnabled :type Boolean))
  (bind _clickablecomponent (Variables|Default|GetClickableComponent))
  (bind _output_get (Variables|Default|SetEnabled NewEnabled))
  (if _output_get
    (Class|ClickableComponent|SetActiveUseContext _clickablecomponent "UC_TurnOff")
    (CallFunction|CheckGases)
    (else
      (Class|ClickableComponent|SetActiveUseContext _clickablecomponent "UC_TurnOn"))))

(event EventBeginPlay
  (Variables|Default|SetChildSlotRef (Class|ChildSlotComponent|MakeReference (Variables|Default|GetOutSlot)))
  (CallFunction|CheckGases)
  (Networking|SwitchHasAuthority
    (:Authority
      (CallFunction|SetGasIdxonServer (Variables|Default|GetGasIdx))
      (CallFunction|SetEnabled (Variables|Default|GetEnabled)))))

(event EventTick
  (params (DeltaSeconds :type Float%20%28single-precision%29))
  (bind _power (Variables|Default|GetPower))
  (bind _availablegases (Variables|Default|GetAvailableGases))
  (bind _gasidx (Variables|Default|GetGasIdx))
  (bind _power_2 (Variables|Default|GetPower))
  (bind _output (Utilities|Array|Get(acopy) _availablegases _gasidx))
  (Networking|SwitchHasAuthority
    (:Authority
      (if (and (Variables|Default|GetEnabled) (Class|PowerComponent|IsAnyPowerAvailable _power_2))
        (Class|PowerComponent|SetEnabled _power true)
        (Class|SlotStatics|AddItemRateDelta (Variables|Default|GetChildSlotRef) _output (* (* (Variables|Default|GetProcessRate) (/ (Variables|/Script/Astro.PowerComponent|GetNetActualLoad _power_2) (Class|PowerComponent|GetDefaultNetPowerOutput _power_2))) (.Value (Utilities|Map|Find (Variables|Default|GetGasDensities) _output))) DeltaSeconds)
        (else
          (Class|PowerComponent|SetEnabled _power false))))))

(event Input|ActionEvents|InputActionUse
  (params (Key :type Key%20Structure :default "None"))
  (:Pressed
    (switch Utilities|FlowControl|Switch|SwitchonEUseContext (Class|ClickableComponent|GetActiveUseContext (Variables|Default|GetClickableComponent))
      (:UC_TurnOn
        (CallFunction|SetEnabled true))
      (:UC_TurnOff
        (CallFunction|SetEnabled false)))))

(fn ConstructionScript)

(fn GetBodySlotLegacy
  (return (Variables|Default|GetBodySlot)))

(fn SetGasIdxonServer
  (params (NewGasIdx :type Integer))
  (bind _output_get (Variables|Default|SetGasIdx NewGasIdx))
  (CallFunction|CheckGases)
  (Rendering|Components|TextRender|SetText (Variables|Default|GetTextRender) (Variables|/Script/Astro.ControlSymbol|GetName (Class|AstroPlayStatics|GetControlSymbolDefault (Utilities|Array|Get(acopy) (Variables|Default|GetAvailableGases) _output_get)))))

(fn CheckGases
  (Utilities|Array|Clear (Variables|Default|GetAvailableGases))
  (Utilities|Map|Clear (Variables|Default|GetGasDensities))
  (for _array_element (Variables|/Script/Astro.AstroPlanet|GetAtmosphericResources (Class|PlanetStatics|GetPlanet self false))
    (if (> (.Density (Utilities|Struct|BreakAtmosphericResource _array_element)) 0.0)
      (Utilities|Array|Add (Variables|Default|GetAvailableGases) (.ResourceItemType (Utilities|Struct|BreakAtmosphericResource _array_element)))
      (Utilities|Map|Add (Variables|Default|GetGasDensities) (.ResourceItemType (Utilities|Struct|BreakAtmosphericResource _array_element)) (.Density (Utilities|Struct|BreakAtmosphericResource _array_element)))))
  (if (>= (Variables|Default|GetGasIdx) (Utilities|Array|Length (Variables|Default|GetAvailableGases)))
    (Networking|SwitchHasAuthority
      (:Authority
        (Variables|Default|SetGasIdx 0)))))

(fn OnRepGasIdx
  (Rendering|Components|TextRender|SetText (Variables|Default|GetTextRender) (Variables|/Script/Astro.ControlSymbol|GetName (Class|AstroPlayStatics|GetControlSymbolDefault (Utilities|Array|Get(acopy) (Variables|Default|GetAvailableGases) (Variables|Default|GetGasIdx))))))