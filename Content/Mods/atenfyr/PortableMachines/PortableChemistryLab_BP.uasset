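; Portable chemistry lab machine that converts up to three slotted input resources into a selected output resource.
; Capsule clicks cycle the recipe through PMActorComponent on the local player controller, relaying client input for SetRecipeIdxOnServer.
; Recipes come from each output's ConstructionRecipe, doubled first ingredients filling two slots, and rewrite slot whitelists and the label.
; While enabled, powered and correctly stocked, authority Tick consumes inputs and produces output, scaled by power load.
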(event OnClicked(Capsule_right)
  (params (TouchedComponent :type Primitive%20Component%20Object%20Reference) (ButtonPressed :type Key%20Structure :default "None"))
  (bind _returnvalue (Class|AstroPlayStatics|GetLocalPlayController))
  (bind _returnvalue_2 (Actor|GetComponentbyClass _returnvalue "/Game/Mods/atenfyr/PortableMachines/PMActorComponent.PMActorComponent_C"))
  (Utilities|IsValid _returnvalue_2
    (:Is%20Valid
      (Default|SetRecipeIdxonOwningClient _returnvalue_2 (CallFunction|ClampRecipeIdx (+ (Variables|Default|GetRecipeIdx) 1)) self))))

(event OnClicked(Capsule_left)
  (params (TouchedComponent :type Primitive%20Component%20Object%20Reference) (ButtonPressed :type Key%20Structure :default "None"))
  (bind _returnvalue (Class|AstroPlayStatics|GetLocalPlayController))
  (bind _returnvalue_2 (Actor|GetComponentbyClass _returnvalue "/Game/Mods/atenfyr/PortableMachines/PMActorComponent.PMActorComponent_C"))
  (Utilities|IsValid _returnvalue_2
    (:Is%20Valid
      (Default|SetRecipeIdxonOwningClient _returnvalue_2 (CallFunction|ClampRecipeIdx (- (Variables|Default|GetRecipeIdx) 1)) self))))

(event Custom|SetEnabled
  (params (NewEnabled :type Boolean))
  (bind _clickablecomponent (Variables|Default|GetClickableComponent))
  (bind _output_get (Variables|Default|SetEnabled NewEnabled))
  (CallFunction|UpdateIndicators _output_get)
  (if _output_get
    (Class|ClickableComponent|SetActiveUseContext _clickablecomponent "UC_TurnOff")
    (else
      (Class|ClickableComponent|SetActiveUseContext _clickablecomponent "UC_TurnOn"))))

(event EventBeginPlay
  (Variables|Default|SetInSlot1_ref (Class|ChildSlotComponent|MakeReference (Variables|Default|GetInSlot1)))
  (Variables|Default|SetInSlot2_ref (Class|ChildSlotComponent|MakeReference (Variables|Default|GetInSlot2)))
  (Variables|Default|SetInSlot3_ref (Class|ChildSlotComponent|MakeReference (Variables|Default|GetInSlot3)))
  (Variables|Default|SetOutSlot_ref (Class|ChildSlotComponent|MakeReference (Variables|Default|GetOutSlot)))
  (Networking|SwitchHasAuthority
    (:Authority
      (CallFunction|SetRecipeIdxonServer (Variables|Default|GetRecipeIdx))
      (CallFunction|SetEnabled (Variables|Default|GetEnabled)))))

(event EventTick
  (params (DeltaSeconds :type Float%20%28single-precision%29))
  (bind _processrate (Variables|Default|GetProcessRate))
  (bind _power (Variables|Default|GetPower))
  (bind _power_2 (Variables|Default|GetPower))
  (bind _returnvalue (Class|PowerComponent|GetDefaultNetPowerOutput _power))
  (bind _netactualload (Variables|/Script/Astro.PowerComponent|GetNetActualLoad _power))
  (bind _returnvalue_2 (/ _netactualload _returnvalue))
  (bind _returnvalue_3 (* _processrate _returnvalue_2))
  (Networking|SwitchHasAuthority
    (:Authority
      (bind _success (CallFunction|AreInputsCorrect))
      (if (Math|Boolean|ANDBoolean (Variables|Default|GetEnabled) (Class|PowerComponent|IsAnyPowerAvailable _power) _success)
        (Class|PowerComponent|SetEnabled _power_2 true)
        (Class|SlotStatics|AddItemRateDelta (Variables|Default|GetOutSlot_ref) (Utilities|Array|Get(acopy) (Utilities|GetClassDefaults (Variables|Default|GetResourceList)) (Variables|Default|GetRecipeIdx)) _returnvalue_3 DeltaSeconds)
        (CallFunction|TakeAllItems DeltaSeconds _returnvalue_3)
        (else
          (Class|PowerComponent|SetEnabled _power_2 false))))))

(event Input|ActionEvents|InputActionUse
  (params (Key :type Key%20Structure :default "None"))
  (:Pressed
    (switch Utilities|FlowControl|Switch|SwitchonEUseContext (Class|ClickableComponent|GetActiveUseContext (Variables|Default|GetClickableComponent))
      (:UC_TurnOn
        (CallFunction|SetEnabled true))
      (:UC_TurnOff
        (CallFunction|SetEnabled false)))))

(fn ConstructionScript)

(fn GetBodySlotLegacy
  (return (Variables|Default|GetBodySlot)))

(fn AreInputsCorrect
  (bind (_in1 _in2 _in3) (CallFunction|GetRequiredInputResources))
  (return (Math|Boolean|ANDBoolean (== _in1 (Class|SlotStatics|GetPrimaryItemTypeClass (Variables|Default|GetInSlot1_ref))) (== _in2 (Class|SlotStatics|GetPrimaryItemTypeClass (Variables|Default|GetInSlot2_ref))) (or (== _in3 (Class|SlotStatics|GetPrimaryItemTypeClass (Variables|Default|GetInSlot3_ref))) (not (Utilities|IsValidClass _in3))))))

(fn TakeAllItems
  (params (Delta%20Time :type Float%20%28single-precision%29) (Rate :type Float%20%28single-precision%29))
  (bind _inslot2_ref (Variables|Default|GetInSlot2_ref))
  (bind _inslot1_ref (Variables|Default|GetInSlot1_ref))
  (bind _inslot3_ref (Variables|Default|GetInSlot3_ref))
  (Class|SlotStatics|TakeItemRateDelta _inslot1_ref (Class|SlotStatics|GetItemTypeClass _inslot1_ref) Rate Delta%20Time 0.0)
  (Class|SlotStatics|TakeItemRateDelta _inslot2_ref (Class|SlotStatics|GetItemTypeClass _inslot2_ref) Rate Delta%20Time 0.0)
  (Class|SlotStatics|TakeItemRateDelta _inslot3_ref (Class|SlotStatics|GetItemTypeClass _inslot3_ref) Rate Delta%20Time 0.0)
  (return))

(fn GetRequiredInputResources
  (bind _resourcelist (Variables|Default|GetResourceList))
  (bind _recipeidx (Variables|Default|GetRecipeIdx))
  (bind _itemtypes (Utilities|GetClassDefaults _resourcelist))
  (bind _output (Utilities|Array|Get(acopy) _itemtypes _recipeidx))
  (bind _constructionrecipe (Utilities|GetClassDefaults _output))
  (bind _ingredients (Utilities|Struct|BreakRecipe _constructionrecipe))
  (bind _output_2 (Utilities|Array|Get(acopy) _ingredients))
  (bind _output_3 (Utilities|Array|Get(acopy) _ingredients 1))
  (bind (_itemtype _count) (Utilities|Struct|BreakItemRecipeIngredient _output_2))
  (bind _itemtype_2 (Utilities|Struct|BreakItemRecipeIngredient _output_3))
  (if (Math|Float|NearlyEqual(Float) _count 2.0 0.5)
    (return _itemtype _itemtype _itemtype_2 _output)
    (else
      (return _itemtype _itemtype_2 (.ItemType (Utilities|Struct|BreakItemRecipeIngredient (Utilities|Array|Get(acopy) _ingredients 2))) _output))))

(fn SetRecipeIdxonServer
  (params (NewRecipeIdx :type Integer))
  (bind _storagechassis (Variables|Default|GetStorageChassis))
  (bind _storagechassis_2 (Variables|Default|GetStorageChassis))
  (bind _storagechassis_3 (Variables|Default|GetStorageChassis))
  (bind _organizationrules (Variables|/Script/Astro.StorageChassisComponent|GetOrganizationRules _storagechassis))
  (bind _organizationrules_2 (Variables|/Script/Astro.StorageChassisComponent|GetOrganizationRules _storagechassis_2))
  (bind _organizationrules_3 (Variables|/Script/Astro.StorageChassisComponent|GetOrganizationRules _storagechassis_3))
  (Variables|Default|SetRecipeIdx NewRecipeIdx)
  (bind (_in1 _in2 _in3 _out) (CallFunction|GetRequiredInputResources))
  (bind _asdynamic_whitelist_organization_rule (Utilities|Casting|CastToDynamicWhitelistOrganizationRule (Utilities|Array|Get(acopy) _organizationrules))
    (:then
      (Utilities|Array|Clear (Variables|/Script/Astro.DynamicWhitelistOrganizationRule|GetItemTypeWhitelist _asdynamic_whitelist_organization_rule))
      (Utilities|Array|Add (Variables|/Script/Astro.DynamicWhitelistOrganizationRule|GetItemTypeWhitelist _asdynamic_whitelist_organization_rule) _in1)
      (Utilities|Array|SetArrayElem _organizationrules 0 _asdynamic_whitelist_organization_rule)
      (Class|DynamicWhitelistOrganizationRule|SetShowIndicators _asdynamic_whitelist_organization_rule (Variables|Default|GetEnabled)))
    (:CastFailed
      _))
  (bind _asdynamic_whitelist_organization_rule_2 (Utilities|Casting|CastToDynamicWhitelistOrganizationRule (Utilities|Array|Get(acopy) _organizationrules_3 1))
    (:then
      (Utilities|Array|Clear (Variables|/Script/Astro.DynamicWhitelistOrganizationRule|GetItemTypeWhitelist _asdynamic_whitelist_organization_rule_2))
      (Utilities|Array|Add (Variables|/Script/Astro.DynamicWhitelistOrganizationRule|GetItemTypeWhitelist _asdynamic_whitelist_organization_rule_2) _in2)
      (Utilities|Array|SetArrayElem _organizationrules_3 1 _asdynamic_whitelist_organization_rule_2)
      (Class|DynamicWhitelistOrganizationRule|SetShowIndicators _asdynamic_whitelist_organization_rule_2 (Variables|Default|GetEnabled)))
    (:CastFailed
      _))
  (bind _asdynamic_whitelist_organization_rule_3 (Utilities|Casting|CastToDynamicWhitelistOrganizationRule (Utilities|Array|Get(acopy) _organizationrules_2 2))
    (:then
      (Utilities|Array|Clear (Variables|/Script/Astro.DynamicWhitelistOrganizationRule|GetItemTypeWhitelist _asdynamic_whitelist_organization_rule_3))
      (if (Utilities|IsValidClass _in3)
        (Utilities|Array|Add (Variables|/Script/Astro.DynamicWhitelistOrganizationRule|GetItemTypeWhitelist _asdynamic_whitelist_organization_rule_3) _in3)
        (else
          (Utilities|Array|Add (Variables|/Script/Astro.DynamicWhitelistOrganizationRule|GetItemTypeWhitelist _asdynamic_whitelist_organization_rule_3) 0)))
      (Utilities|Array|SetArrayElem _organizationrules_2 2 _asdynamic_whitelist_organization_rule_3)
      (Class|DynamicWhitelistOrganizationRule|SetShowIndicators _asdynamic_whitelist_organization_rule_3 (Variables|Default|GetEnabled)))
    (:CastFailed
      _))
  (Class|StorageChassisComponent|AuthorityApplyOrganizationRules (Variables|Default|GetStorageChassis))
  (Rendering|Components|TextRender|SetText (Variables|Default|GetTextRender) (Variables|/Script/Astro.ControlSymbol|GetName (Class|AstroPlayStatics|GetControlSymbolDefault _out))))

(fn UpdateIndicators
  (params (State :type Boolean))
  (Networking|SwitchHasAuthority
    (:Authority
      (for _array_element (Variables|/Script/Astro.StorageChassisComponent|GetOrganizationRules (Variables|Default|GetStorageChassis))
        (bind _asdynamic_whitelist_organization_rule (Utilities|Casting|CastToDynamicWhitelistOrganizationRule _array_element))
        (Class|DynamicWhitelistOrganizationRule|SetShowIndicators _asdynamic_whitelist_organization_rule State)
        (Class|SlotOrganizationRule|SetEnabled _array_element State true)))))

(fn ClampRecipeIdx
  (params (TestRecipeIdx :type Integer))
  (bind _resourcelist (Variables|Default|GetResourceList))
  (bind _itemtypes (Utilities|GetClassDefaults _resourcelist))
  (bind _returnvalue (Utilities|Array|Length _itemtypes))
  (if (< TestRecipeIdx 0)
    (return (+ TestRecipeIdx _returnvalue))
    (elif (>= TestRecipeIdx _returnvalue)
      (return (- TestRecipeIdx _returnvalue))
      (else
        (return TestRecipeIdx)))))