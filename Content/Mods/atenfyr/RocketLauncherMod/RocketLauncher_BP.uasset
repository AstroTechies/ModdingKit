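; Astroneer mod rocket launcher item that consumes slotted fuel to fire rockets, with explosive power set by fuel type.
; Use spawns the rocket and sound, inherits launcher velocity, sphere-traces for clear spawn space and raises a mission event.
; Rockets follow the barrel, or a mouse-trace direction sent through a player-controller component when on a backpack aux slot or in a VTOL.
; Tick updates velocity and aim, hiding fuel indicators on aux slots.
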(event Custom|PlaySounds
  (params (Location :type Vector))
  (bind _returnvalue (Class|AstroGameUserSettings|GetAstroGameUserSettings))
  ;[1 1 1] Normally, Wwise is used for sound (and to provide randomization of which effect is played), but the installation procedure for Wwise is difficult and may not be feasible for some folks, so for this example we just play one sound and forget about the rest
  (Audio|PlaySoundatLocation "/Game/Mods/atenfyr/RocketLauncherMod/Fire.Fire" Location "0, 0, 0" (* (Variables|/Script/Astro.AstroGameUserSettings|GetSoundFXVol _returnvalue) (Variables|/Script/Astro.AstroGameUserSettings|GetMasterVol _returnvalue)) 1.0 0.0 0 0 self))

(event Custom|AdjustHolograms
  (params (Rule :type Whitelist%20Organization%20Rule%20Object%20Reference))
  ;[1 1 1] In Astroneer, items in the backpack have no resource hologram
  (if (not (Class|AstroStatics|IsDedicatedServer))
    (Class|WhitelistOrganizationRule|SetShowIndicators Rule (not (CallFunction|AreWeonAuxSlot)))))

(event Custom|FetchMouseDirection
  (bind _returnvalue (Class|AstroPlayStatics|GetLocalPlayController))
  (bind _returnvalue_2 (Class|AstroPlayStatics|GetLocalPlayController))
  (bind (_worldlocation _worlddirection _returnvalue_3) (Game|Player|ConvertMouseLocationToWorldSpace _returnvalue_2))
  (if (CallFunction|ShouldRelyonMouseDirection)
    (if _returnvalue_3
      (bind (_outhit _returnvalue_4) (Class|KismetSystemLibrary|LineTraceSinglebyProfile _worldlocation (+ _worldlocation (* _worlddirection 1e+05)) "BlockAllDynamic" false 0 "None" true))
      (if _returnvalue_4
        (CallFunction|SetMouseDirection (CallFunction|GetProjectileLookatVector (.ImpactPoint (Collision|BreakHitResult _outhit))) _returnvalue)
        (else
          (CallFunction|SetMouseDirection (CallFunction|GetProjectileLookatVector (+ _worldlocation (* _worlddirection 1e+04))) _returnvalue))))))

(event Custom|OnSlotRelease
  (params (NewOwner :type Boolean))
  ;[1 1 1] Reset aux slot status when slot changes
  (Variables|Default|SetIsOnAuxSlot false))

(event Custom|OnSlotPlace
  ;[1 1 1] Reset aux slot status when slot changes
  (Variables|Default|SetIsOnAuxSlot false))

(event Custom|SpawnProjectile
  (params (Location :type Vector) (Velocity :type Vector) (Power :type Float%20%28single-precision%29))
  (bind _returnvalue (Game|SpawnActorfromClass "/Game/Mods/atenfyr/RocketLauncherMod/Rocket.Rocket_C" (Math|Transform|MakeTransform Location "0, 0, 0" "1,1,1") "AlwaysSpawn" 0 0))
  (Variables|/Script/Astro.ExplosiveComponent|SetPower (Variables|/Game/Mods/atenfyr/RocketLauncherMod/Rocket.Rocket_C|GetExplosive _returnvalue) Power)
  (Game|Components|ProjectileMovement|SetVelocityinLocalSpace (Variables|/Game/Mods/atenfyr/RocketLauncherMod/Rocket.Rocket_C|GetProjectileMovement _returnvalue) Velocity)
  (CallFunction|PlaySounds Location))

(event EventBeginPlay
  (bind _slotscomponent (Variables|Default|GetSlotsComponent))
  (Variables|Default|SetFuelSlotRef (Class|SlotsComponent|MakeReference _slotscomponent "FuelSlot"))
  (Variables|Default|SetBodySlotRef (Class|SlotsComponent|MakeReference _slotscomponent "BodySlot"))
  (bind _aswhitelist_organization_rule (Utilities|Casting|CastToWhitelistOrganizationRule (Class|StorageChassisComponent|FindRulebyName (Variables|Default|GetStorageChassis) "FuelRule")))
  (Variables|Default|SetRule _aswhitelist_organization_rule)
  (Variables|Default|SetValidFuels (CallFunction|GetValidFuels))
  (Variables|Default|SetLocationLastTick (Transformation|GetWorldLocation (Variables|Default|GetStaticMeshComponent)))
  ;[1 1 1] Reset aux slot status when slot changes
  (EventDispatchers|BindEventtoOnReleasedfromSlot (delegate Custom|OnSlotRelease))
  (EventDispatchers|BindEventtoOnPlacedinSlot (delegate Custom|OnSlotPlace)))

(event EventTick
  (params (DeltaSeconds :type Float%20%28single-precision%29))
  (bind _staticmeshcomponent (Variables|Default|GetStaticMeshComponent))
  (bind _returnvalue (Transformation|GetWorldLocation _staticmeshcomponent))
  ;[1 1 1] In Astroneer, items in the backpack have no resource hologram
  (CallFunction|AdjustHolograms (Variables|Default|GetRule))
  (Variables|Default|SetVelocityThisTick (/ (- _returnvalue (Variables|Default|GetLocationLastTick)) DeltaSeconds))
  (Variables|Default|SetLocationLastTick _returnvalue)
  ;[1 1 1] If it's been more than 2 seconds since the last mouse position update, we revert to the normal mode since it is most definitely not accurate anymore
  (bind _output_get (Variables|Default|SetTimeSinceLastMouseChange (+ (Variables|Default|GetTimeSinceLastMouseChange) DeltaSeconds)))
  (if (> _output_get 2.0)
    (Variables|Default|SetIsOnAuxSlot false))
  (CallFunction|FetchMouseDirection))

(event Input|ActionEvents|InputActionUse
  (params (Key :type Key%20Structure))
  (bind _projectile_direction (CallFunction|GetProjectileDirection))
  (bind _barrel (Variables|Default|GetBarrel))
  (bind _returnvalue (Transformation|GetWorldLocation _barrel))
  (:Pressed
    (bind (_hasfuel _power _fuel_actor) (CallFunction|AnalyzeFuel))
    (if _hasfuel
      (Class|SlotStatics|TakeItemRateDelta (Variables|Default|GetFuelSlotRef) (CallFunction|GetItemTypefromPhysicalItem _fuel_actor) 1.0 1.0) ; Use up the fuel (you can also use Destroy Slot Item here)
      (CallFunction|SpawnProjectile (+ _returnvalue (* _projectile_direction (CallFunction|FindSafeDistanceforProjectiletoSpawn _returnvalue _projectile_direction))) (+ (* _projectile_direction 7.5e+03) (Variables|Default|GetVelocityThisTick)) _power) ; Spawn the projectile on server and all clients (smooth movement)
      (Class|AstroMissionsManager|AuthorityRaiseMissionEvent (Class|AstroStatics|GetAstroMissionsManager) "Custom" 0 0 1.0 "None" "RocketLauncherFire") ; Progresses every mission with the custom tag RocketLauncherFire by 1
    )))

(fn ConstructionScript)

(fn AnalyzeFuel
  (bind _slotscomponent (Variables|Default|GetSlotsComponent))
  (bind _fuelslotref (Variables|Default|GetFuelSlotRef))
  (bind _returnvalue (Class|SlotsComponent|GetSlotPrimaryItem _slotscomponent _fuelslotref))
  (bind _returnvalue_2 (Utilities|GetClass _returnvalue))
  (Utilities|IsValid _returnvalue
    (:Is%20Valid
      (if (Utilities|Array|ContainsItem (Variables|Default|GetValidFuels) _returnvalue_2)
        (Utilities|FlowControl|Sequence
          (:then_0
            (switch string (Utilities|GetClassDisplayName _returnvalue_2) ; Add different kinds of fuel here
              (:Default
                (return false 0.0 _returnvalue))
              (:ResourceNugget_ExplosivePowder_C
                (return true 1.0 _returnvalue))
              (:ResourceNugget13_C
                (return true 2e+01 _returnvalue)))))
        (else
          _)))
    (:Is%20Not%20Valid
      _))
  (return false 0.0 0))

(fn GetBodySlotLegacy
  (return (Variables|Default|GetBodySlot)))

(fn GetItemTypefromPhysicalItem
  (params (PhysicalItem :type Physical%20Item%20Object%20Reference))
  (return (Variables|/Script/Astro.ItemComponent|GetItemType (Actor|GetComponentbyClass PhysicalItem "/Script/Astro.ItemComponent"))))

(fn AreWeonAuxSlot
  (bind _returnvalue (Class|AstroPlayStatics|GetLocalAstroCharacter))
  (bind _returnvalue_2 (Class|AstroCharacter|GetBackpack _returnvalue))
  (bind _returnvalue_3 (Actor|GetComponentbyClass _returnvalue_2 "/Script/Astro.SlotsComponent"))
  (Utilities|IsValid _returnvalue_3
    (:Is%20Valid
      (for _array_element (Variables|/Script/Astro.SlotsComponent|GetSlots _returnvalue_3)
        (if (Class|SlotStatics|IsSlotAnAuxSlot)
          (if (== (Class|SlotsComponent|GetSlotPrimaryItem _returnvalue_3 (Class|SlotsComponent|MakeReference _returnvalue_3 (.Name (Utilities|Struct|BreakSlot _array_element)))) self)
            (return true)))))
    (:Is%20Not%20Valid
      _))
  (return false))

(fn GetValidFuels
  (for _array_element (Utilities|GetClassDefaults (Variables|/Script/Astro.WhitelistOrganizationRule|GetItemTypeWhitelist (Variables|Default|GetRule)))
    (Utilities|Array|Add (LocalVariables|GetCurrentValidItems) (.PickupActor (Utilities|GetClassDefaults _array_element))))
  (return (LocalVariables|GetCurrentValidItems)))

(fn GetProjectileLookatVector
  (params (Impact%20Point :type Vector))
  (return (Math|Vector|Normalize (- Impact%20Point (Transformation|GetWorldLocation (Variables|Default|GetBarrel))))))

(fn GetProjectileDirection
  (if (and (or (Variables|Default|GetIsOnAuxSlot) (CallFunction|ShouldRelyonMouseDirection)) (Math|Vector|NotEqual(Vector) (Variables|Default|GetMouseDirection) "0, 0, 0" 0.0001))
    (return (Variables|Default|GetMouseDirection))
    (else
      (return (Math|Vector|GetUpVector (Variables|Default|GetBarrel))))))

(fn SetMouseDirection
  (params (Mouse%20Direction :type Vector) (Controller :type Play%20Controller%20Object%20Reference))
  (bind _returnvalue (Actor|GetComponentbyClass Controller "/Game/Mods/atenfyr/RocketLauncherMod/RocketLauncherClientComponent.RocketLauncherClientComponent_C"))
  (Utilities|IsValid _returnvalue
    (:Is%20Valid
      (Default|SetMouseDirection _returnvalue Mouse%20Direction self))))

(fn FindSafeDistanceforProjectiletoSpawn
  (params (Starting%20Location :type Vector) (Starting%20Direction :type Vector))
  (LocalVariables|SetCurrentTally 1e+02)
  (while true
    (bind _returnvalue (Class|KismetSystemLibrary|SphereTraceSinglebyProfile (+ Starting%20Location (* Starting%20Direction (+ (LocalVariables|GetCurrentTally) -5e+01))) (+ Starting%20Location (* Starting%20Direction (+ (LocalVariables|GetCurrentTally) 5e+01))) 2e+01 "BlockAllDynamic" false 0 "None" true))
    (if _returnvalue
      (if (> (LocalVariables|GetCurrentTally) 6e+02)
        (return 1.0)
        (else
          (LocalVariables|SetCurrentTally (+ (LocalVariables|GetCurrentTally) 1e+02))))
      (else
        (return (LocalVariables|GetCurrentTally))))))

(fn ShouldRelyonMouseDirection
  (bind _asseat_base (Utilities|Casting|CastToSeatBase (Variables|/Script/Astro.AstroCharacter|GetAttachOwner (Class|AstroPlayStatics|GetLocalAstroCharacter)))
    (:then
      (Utilities|Casting|CastToVtolItem (Class|SeatBase|GetVehicleSlottedto _asseat_base)
        (:then
          (LocalVariables|SetIsInsideVTOL true))
        (:CastFailed
          _)))
    (:CastFailed
      _))
  (return (or (CallFunction|AreWeonAuxSlot) (LocalVariables|GetIsInsideVTOL))))