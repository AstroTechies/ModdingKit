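; Canister clone from the RocketLauncherMod that spawns as a drum pre-filled with Explosive Powder.
; On BeginPlay it fills its item component to capacity with Explosive Powder, guarded by a flag so the initial fill runs only once.
; It overwrites its default description around BeginPlay and again every Tick to keep the custom text in place.
; Pickup, drop and hit events only forward to the parent class.
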(event EventBeginPlay
  (CallFunction|ResetDescription)
  (|CallParentFunction)
  (CallFunction|InitFill (Variables|/Script/Astro.ItemComponent|GetCapacity (Variables|Default|GetItemComponent)))
  (CallFunction|ResetDescription))

(event EventTick
  (params (DeltaSeconds :type Float%20%28single-precision%29))
  (|CallParentFunction DeltaSeconds)
  (CallFunction|ResetDescription))

(event EventPickedUpfromWorld
  (|CallParentFunction))

(event EventDroppedinWorld
  (params (Component :type Primitive%20Component%20Object%20Reference) (NewTerrainComponent :type Boolean) (Point :type Vector%20%28by%20ref%29 :default "0, 0, 0") (Normal :type Vector%20%28by%20ref%29 :default "0, 0, 0"))
  (|CallParentFunction Component NewTerrainComponent Point Normal))

(event Collision|EventHit
  (params (MyComp :type Primitive%20Component%20Object%20Reference) (Other :type Actor%20Object%20Reference) (OtherComp :type Primitive%20Component%20Object%20Reference) (bSelfMoved :type Boolean) (HitLocation :type Vector :default "0, 0, 0") (HitNormal :type Vector :default "0, 0, 0") (NormalImpulse :type Vector :default "0, 0, 0") (Hit :type Hit%20Result%20Structure%20%28by%20ref%29))
  (|CallParentFunction MyComp Other OtherComp bSelfMoved HitLocation HitNormal NormalImpulse Hit))

(fn ConstructionScript
  (|CallParentFunction))

(fn InitFill
  (params (Count :type Float%20%28single-precision%29))
  (if (not (Variables|Default|GetHasAlreadyInitiallyFilled))
    (Class|ItemComponent|SetItem (Variables|Default|GetItemComponent) "/Game/Items/ItemTypes/Composites/ExplosivePowder.ExplosivePowder_C" (Class|ItemStatics|AmountfromRecipe Count) false)
    (Variables|Default|SetHasAlreadyInitiallyFilled true)))

(fn ResetDescription
  (Variables|Default|SetDefaultDescription "Pre-filled drum that holds up to 64 nuggets of Explosive Powder."))